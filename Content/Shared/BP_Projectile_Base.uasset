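; Base projectile Blueprint that handles the sound and particle effects for firing, flight and impact.
; On BeginPlay it plays a launch sound, attaches a flight sound to the root and spawns a muzzle effect facing the actor's forward vector.
; OnSpawnProjectileHitFx plays the impact sound and effect at the given hit location.
; Each asset is validity-checked, and the graph contains no movement or damage logic.
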(event EventBeginPlay
  (Utilities|FlowControl|Sequence
    (:then_0
      (bind _projectilesound (Variables|Default|GetProjectileSound)
        (:then
          (Audio|PlaySoundatLocation _projectilesound (Transformation|GetActorLocation) "0, 0, 0" 1.0 1.0 0.0 0 0 0 0))
        (:else)))
    (:then_1
      (bind _projectileflysound (Variables|Default|GetProjectileFlySound)
        (:then
          (Audio|SpawnSoundAttached _projectileflysound (Variables|Transformation|GetRootComponent) "None" "0, 0, 0" "0, 0, 0" "KeepRelativeOffset" true 1.0 1.0 0.0 0 0))
        (:else)))
    (:then_2
      (bind _projectilemuzzlefx (Variables|Default|GetProjectileMuzzleFx)
        (:then
          (Niagara|SpawnSystematLocation _projectilemuzzlefx (Transformation|GetActorLocation) (Math|Conversions|RotationFromXVector (Transformation|GetActorForwardVector))))
        (:else)))))

(event EventOnSpawnProjectileHitFx
  (params (HitLocation :type Vector%20%28by%20ref%29 :default "0, 0, 0"))
  (Utilities|FlowControl|Sequence
    (:then_0
      (bind _projectileimpactsound (Variables|Default|GetProjectileImpactSound)
        (:then
          (Audio|PlaySoundatLocation _projectileimpactsound HitLocation "0, 0, 0" 1.0 1.0 0.0 0 0 0 0))
        (:else)))
    (:then_1
      (bind _projectileimpactfx (Variables|Default|GetProjectileImpactFX)
        (:then
          (Niagara|SpawnSystematLocation _projectileimpactfx HitLocation))
        (:else)))))

(fn ConstructionScript)