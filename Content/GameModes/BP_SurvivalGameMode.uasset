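; Survival game mode Blueprint that handles on-screen presentation of the wave-based match, reacting to game mode state changes bound at BeginPlay.
; Wave states spawn text or countdown widgets through two helper functions, and the final wave also changes the enemy spawn delay and shows a "Last Wave" banner.
; Victory or player death clears widgets, fades the camera to black, then async-loads the win or lose screen class and adds it to the viewport.
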(event Custom|OnSurvivalGameModeStateChanged_Event
  (params (CurrentState :type EWarriorSurvivalGameModeState%20Enum :default "WaitSpawnNewWave"))
  (switch Utilities|FlowControl|Switch|SwitchonEWarriorSurvivalGameModeState CurrentState
    (:WaitSpawnNewWave
      (CallFunction|CreateWaveWidgetwithCountDown "New Wave is Coming In" (Variables|Default|GetSpawnNewWaveWaitTime)))
    (:SpawningNewWave
      (CallFunction|CreateWaveWidget (Utilities|Text|FormatText "Wave {CurrentWaveCount}" (Variables|Default|GetCurrentWaveCount)))
      (if (== (Variables|Default|GetCurrentWaveCount) (Variables|Default|GetTotalWavesToSpawn))
        (Variables|Default|SetSpawnEnemiesDelayTime 4.0)
        (Utilities|FlowControl|Delay 2.0)
        (CallFunction|CreateWaveWidget "Last Wave")))
    (:WaveCompleted
      (CallFunction|CreateWaveWidgetwithCountDown (Utilities|Text|FormatText "Wave {CurrentWaveCount}" (Variables|Default|GetCurrentWaveCount)) (Variables|Default|GetWaveCompletedWaitTime)))
    (:AllWavesDone
      (Utilities|FlowControl|Delay 1.5)
      (Viewport|RemoveAllWidgets)
      (CameraFades|StartCameraFade :self (Game|GetPlayerCameraManager 0) :ToAlpha 1.0 :Duration 3.0 :bHoldWhenFinished true)
      (Utilities|FlowControl|Delay 3.0)
      (bind _class (Utilities|AsyncLoadClassAsset "/Game/Widgets/GameModeWidgets/WBP_WinScreen.WBP_WinScreen_C")
        (:Completed
          (bind _asuser_widget (Utilities|Casting|CastToUserWidgetClass _class))
          (bind _returnvalue (UserInterface|CreateWidget _asuser_widget))
          (UserInterface|Viewport|AddtoViewport _returnvalue 0))))
    (:PlayerDied
      (Viewport|RemoveAllWidgets)
      (CameraFades|StartCameraFade :self (Game|GetPlayerCameraManager 0) :ToAlpha 1.0 :Duration 2.0 :bHoldWhenFinished true)
      (Utilities|FlowControl|Delay 2.0)
      (bind _class_2 (Utilities|AsyncLoadClassAsset "/Game/Widgets/GameModeWidgets/WBP_LoseScreen.WBP_LoseScreen_C")
        (:Completed
          (bind _asuser_widget_2 (Utilities|Casting|CastToUserWidgetClass _class_2))
          (bind _returnvalue_2 (UserInterface|CreateWidget _asuser_widget_2))
          (UserInterface|Viewport|AddtoViewport _returnvalue_2 0))))))

(event EventBeginPlay
  (EventDispatchers|AssignOnSurvivalGameModeStateChanged (delegate Custom|OnSurvivalGameModeStateChanged_Event)))

(event EventTick
  (params (DeltaSeconds :type Float%20%28single-precision%29)))

(fn ConstructionScript)

(fn CreateWaveWidgetwithCountDown
  (params (InTextContent :type Text) (InTotalCountDownTime :type Float%20%28double-precision%29))
  (bind _returnvalue (UserInterface|CreateWidget "/Game/Widgets/GameModeWidgets/WBP_WaveTextWithCountDown.WBP_WaveTextWithCountDown_C"))
  (UserInterface|Viewport|AddtoViewport _returnvalue 0)
  (Rendering|Components|TextRender|SetText (Variables|/Game/Widgets/GameModeWidgets/WBP_WaveTextWithCountDown.WBP_WaveTextWithCountDown_C|GetTextBlock_Wave _returnvalue) InTextContent)
  (Default|StartCountDown _returnvalue InTotalCountDownTime))

(fn CreateWaveWidget
  (params (InText :type Text))
  (bind _returnvalue (UserInterface|CreateWidget "/Game/Widgets/GameModeWidgets/WBP_WaveTextWithNoCountDown.WBP_WaveTextWithNoCountDown_C"))
  (UserInterface|Viewport|AddtoViewport _returnvalue 0)
  (Rendering|Components|TextRender|SetText (Variables|/Game/Widgets/GameModeWidgets/WBP_WaveTextWithNoCountDown.WBP_WaveTextWithNoCountDown_C|GetTextBlock_Wave _returnvalue) InText))